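; End-of-game platform actor that sends the player back to the Menu level.
; When BP_PhysicsPlayer overlaps its box, it calls the player's FadeToBlack, waits briefly, then opens the menu.
; The construction script gives the platform a dynamic M_EndGame material.
; Its own FadeToBlack timeline, not called here, and an unconnected color-lerp timeline target that material with parameter names left as None.
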(event `FadeToBlack`
  (bind (_direction _data) (`Timeline|FadeToNoOpacity`)
    (:`Update`
      (`MaterialInstanceDynamic.SetScalarParameterValue` (`self.FadeDMI`) "None" _data))))

(event `self.ReceiveBeginPlay`)

(event `self.ReceiveActorBeginOverlap`
  (params (OtherActor :type "Actor Object Reference")))

(event `self.ReceiveTick`
  (params (DeltaSeconds :type "Float (single-precision)")))

(event `self.Box.OnComponentBeginOverlap`
  (params (OtherActor :type "Actor Object Reference") (OtherComp :type "PrimitiveComponent Object Reference") (OtherBodyIndex :type Integer) (bFromSweep :type Boolean) (SweepResult :type "HitResult Structure (by ref)"))
  (bind _asbp_physics_player (cast `/Game/Blueprints/Character/BP_PhysicsPlayer` OtherActor))
  (`/Game/Blueprints/Character/BP_PhysicsPlayer.FadeToBlack` _asbp_physics_player)
  (`KismetSystemLibrary.Delay` 1.0)
  (`GameplayStatics.OpenLevel` "Menu"))

(fn `UserConstructionScript`
  (bind _returnvalue (`PrimitiveComponent.CreateDynamicMaterialInstance` (`self.Platform`) 0 "/Game/Materials/M_EndGame.M_EndGame"))
  (set `self.FadeDMI` _returnvalue))