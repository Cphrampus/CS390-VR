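; BP_Button is a menu button whose Select event decides its action from the placed instance's object name.
; The Play and Other buttons call FadeToBlack on the BP_MenuPlayer pawn, wait briefly, then open their level.
; The Music button plays the starter music once through a DoOnce, and any other name quits the game.
; Every action requires the player pawn to cast to BP_MenuPlayer.
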(event `self.ReceiveBeginPlay`)

(event `self.ReceiveActorBeginOverlap`
  (params (OtherActor :type "Actor Object Reference")))

(event `self.ReceiveTick`
  (params (DeltaSeconds :type "Float (single-precision)")))

(event `Select`
  (bind _returnvalue (`KismetSystemLibrary.GetObjectName` self))
  (bind _asbp_menu_player (cast `/Game/Blueprints/Character/BP_MenuPlayer` (`GameplayStatics.GetPlayerPawn` 0)))
  (if (`KismetStringLibrary.EqualEqual_StrStr` _returnvalue "BP_ButtonPLay")
    (`/Game/Blueprints/Character/BP_MenuPlayer.FadeToBlack` _asbp_menu_player)
    (`KismetSystemLibrary.Delay` 1.0)
    (`GameplayStatics.OpenLevel` "PhysicsPlayground")
    (elif (`KismetStringLibrary.EqualEqual_StrStr` _returnvalue "BP_ButtonOther")
      (`/Game/Blueprints/Character/BP_MenuPlayer.FadeToBlack` _asbp_menu_player)
      (`KismetSystemLibrary.Delay` 1.0)
      (`GameplayStatics.OpenLevel` "Other")
      (elif (`KismetStringLibrary.EqualEqual_StrStr` _returnvalue "BP_ButtonMusic")
        (`/Engine/EditorBlueprintResources/StandardMacros.DoOnce` false
          (:`Completed`
            (`GameplayStatics.PlaySoundAtLocation` "/Game/MobileStarterContent/Audio/Starter_Music01.Starter_Music01")))
        (else
          (`KismetSystemLibrary.QuitGame` null "Quit"))))))

(fn `UserConstructionScript`)