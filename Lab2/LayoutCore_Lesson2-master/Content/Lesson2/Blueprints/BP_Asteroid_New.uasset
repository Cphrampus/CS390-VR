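; Lesson asteroid actor that homes in on the player pawn and explodes on any actor overlap.
; Each Tick it moves a fixed, frame-rate-dependent step toward the player with sweep, applies the stored rotation, then re-randomizes it, giving an erratic tumble.
; Overlap destroys it, spawns a green explosion at its location and plays the sound at world origin.
; BeginPlay shows a debug string and seeds the first random rotation.
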(event `/Game/Lesson2/Blueprints/BP_Asteroid.ReceiveActorBeginOverlap`
  (params (OtherActor :type "Actor Object Reference"))
  (`self.K2_DestroyActor`)
  (`GameplayStatics.SpawnEmitterAtLocation` "/Game/Lesson2/Effects/P_Explosion_Green.P_Explosion_Green" (`self.K2_GetActorLocation`))
  (`GameplayStatics.PlaySoundAtLocation` "/Game/EpicsMobileStarterContent/Audio/Explosion01.Explosion01"))

(event `/Game/Lesson2/Blueprints/BP_Asteroid.ReceiveBeginPlay`
  (`/Game/LayoutAssets/Utility/LayoutVRUtilityFunctions.Draw VR Debug String` "Testing" (+ (`self.K2_GetActorLocation`) (0.0 0.0 200.0)) 10.0)
  (set `self.Rotation` (`KismetMathLibrary.MakeRotator` (`KismetMathLibrary.RandomFloatInRange` 0.0 360.0) (`KismetMathLibrary.RandomFloatInRange` 0.0 360.0) (`KismetMathLibrary.RandomFloatInRange` 0.0 360.0))))

(event `/Game/Lesson2/Blueprints/BP_Asteroid.ReceiveTick`
  (params (DeltaSeconds :type "Float (single-precision)"))
  ;[1 1 1] Make Asteroid move toward player
  (`self.K2_AddActorWorldOffset` (* (`KismetMathLibrary.GetDirectionVector` (`self.K2_GetActorLocation`) (`self.K2_GetActorLocation` (`GameplayStatics.GetPlayerPawn` 0))) 5.0) true)
  (`self.K2_AddActorWorldRotation` (`self.Rotation`))
  (set `self.Rotation` (`KismetMathLibrary.MakeRotator` (`KismetMathLibrary.RandomFloatInRange` 0.0 360.0) (`KismetMathLibrary.RandomFloatInRange` 0.0 360.0) (`KismetMathLibrary.RandomFloatInRange` 0.0 360.0))))

(fn `UserConstructionScript`)