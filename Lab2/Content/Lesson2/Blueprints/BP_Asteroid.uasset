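; Asteroid actor that homes in on the player pawn and explodes when it overlaps any actor.
; BeginPlay picks one of three meshes and a random rotation, and prints a test debug string.
; Tick sweeps it toward player 0 at a random step size and applies a rotation re-randomized every frame.
; Overlap plays an explosion sound at world origin, destroys the actor and spawns a random particle effect at its location.
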(event `self.ReceiveActorBeginOverlap`
  (params (OtherActor :type "Actor Object Reference"))
  (bind _returnvalue (`self.K2_GetActorLocation`))
  ;[1 1 1] Random Particle system on hit
  (`GameplayStatics.PlaySoundAtLocation` "/Game/MobileStarterContent/Audio/Explosion02.Explosion02")
  (`self.K2_DestroyActor`)
  (switch `int` (`KismetMathLibrary.RandomIntegerInRange` 0 8)
    (:`0`
      (`GameplayStatics.SpawnEmitterAtLocation` "/Game/Lesson2/Effects/P_Explosion_Fuchsia.P_Explosion_Fuchsia" _returnvalue))
    (:`1`
      (`GameplayStatics.SpawnEmitterAtLocation` "/Game/EpicsMobileStarterContent/Particles/P_Explosion.P_Explosion" _returnvalue))
    (:`2`
      (`GameplayStatics.SpawnEmitterAtLocation` "/Game/Lesson2/Effects/P_Explosion_Green.P_Explosion_Green" _returnvalue))
    (:`3`
      (`GameplayStatics.SpawnEmitterAtLocation` "/Game/MobileStarterContent/Particles/P_Sparks.P_Sparks" _returnvalue))
    (:`4`
      (`GameplayStatics.SpawnEmitterAtLocation` "/Game/Lesson2/Effects/P_Explosion_Orange.P_Explosion_Orange" _returnvalue))
    (:`5`
      (`GameplayStatics.SpawnEmitterAtLocation` "/Game/Lesson2/Effects/P_Explosion_Red.P_Explosion_Red" _returnvalue))
    (:`6`
      (`GameplayStatics.SpawnEmitterAtLocation` "/Game/EpicsMobileStarterContent/Particles/P_Fire.P_Fire" _returnvalue))
    (:`7`
      (`GameplayStatics.SpawnEmitterAtLocation` "/Game/EpicsMobileStarterContent/Particles/P_Ambient_Dust.P_Ambient_Dust" _returnvalue))
    (:`8`
      (`GameplayStatics.SpawnEmitterAtLocation` "/Game/EpicsMobileStarterContent/Particles/P_Smoke.P_Smoke" _returnvalue))))

(event `self.ReceiveBeginPlay`
  (bind _staticmesh (`self.StaticMesh`))
  (`/Game/LayoutAssets/Utility/LayoutVRUtilityFunctions.Draw VR Debug String` "Testing" (0.0 0.0 0.0) 10.0)
  ;[1 1 1] Rotation
  (set `self.Rotation` (`KismetMathLibrary.MakeRotator` (`KismetMathLibrary.RandomFloatInRange` 0.0 360.0) (`KismetMathLibrary.RandomFloatInRange` 0.0 360.0) (`KismetMathLibrary.RandomFloatInRange` 0.0 360.0)))
  ;[1 1 1] Randomly set the mesh of the asteroid
  (switch `int` (`KismetMathLibrary.RandomIntegerInRange` 0 2)
    (:`0`
      (`StaticMeshComponent.SetStaticMesh` _staticmesh "/Game/Lesson2/Effects/Meshes/Asteroid_gib_001.Asteroid_gib_001"))
    (:`1`
      (`StaticMeshComponent.SetStaticMesh` _staticmesh "/Game/Lesson2/Effects/Meshes/Asteroid_gib_002.Asteroid_gib_002"))
    (:`2`
      (`StaticMeshComponent.SetStaticMesh` _staticmesh "/Game/Lesson2/Effects/Meshes/Asteroid_gib_003.Asteroid_gib_003"))))

(event `self.ReceiveTick`
  (params (DeltaSeconds :type "Float (single-precision)"))
  ;[1 1 1] Make Asteroid move toward player
  (`self.K2_AddActorWorldOffset` (* (`KismetMathLibrary.GetDirectionVector` (`self.K2_GetActorLocation`) (`self.K2_GetActorLocation` (`GameplayStatics.GetPlayerPawn` 0))) (`KismetMathLibrary.Conv_IntToDouble` (`KismetMathLibrary.RandomIntegerInRange` 1 5))) true)
  (`self.K2_AddActorWorldRotation` (`self.Rotation`))
  (set `self.Rotation` (`KismetMathLibrary.MakeRotator` (`KismetMathLibrary.RandomFloatInRange` 0.0 360.0) (`KismetMathLibrary.RandomFloatInRange` 0.0 360.0) (`KismetMathLibrary.RandomFloatInRange` 0.0 360.0))))

(fn `UserConstructionScript`)