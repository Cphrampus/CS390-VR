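; BP_ScoreAddition is a floating score popup actor that displays a score change as 3D text, then destroys itself.
; The construction script sets the text from ScoreAddition and colors it red for negative values.
; On BeginPlay, the Animation timeline drives height above the start location and font size, rotating the actor to face the player pawn on each update.
; The actor is destroyed when the timeline finishes.
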(event `self.ReceiveBeginPlay`
  (bind (_startinglocation_x _startinglocation_y _startinglocation_z) (`KismetMathLibrary.BreakVector` (`self.StartingLocation`)))
  (set `self.StartingLocation` (`self.K2_GetActorLocation`))
  (bind (_direction _opacity _height _fontsize) (`Timeline|Animation`)
    (:`Update`
      (`self.K2_SetActorLocationAndRotation` (`KismetMathLibrary.MakeVector` _startinglocation_x _startinglocation_y (+ _startinglocation_z (* _height 100.0))) (`KismetMathLibrary.FindLookAtRotation` (`self.K2_GetActorLocation`) (`self.K2_GetActorLocation` (`GameplayStatics.GetPlayerPawn` 0))))
      (`TextRenderComponent.SetWorldSize` (`self.TextRender`) (* _fontsize 36.0)))
    (:`Finished`
      (`self.K2_DestroyActor`))))

(event `self.ReceiveActorBeginOverlap`
  (params (OtherActor :type "Actor Object Reference")))

(event `self.ReceiveTick`
  (params (DeltaSeconds :type "Float (single-precision)")))

(fn `UserConstructionScript`
  (`TextRenderComponent.K2_SetText` (`self.TextRender`) (`KismetTextLibrary.Conv_IntToText` (`self.ScoreAddition`)))
  (if (< (`self.ScoreAddition`) 0)
    (`TextRenderComponent.SetTextRenderColor` (`self.TextRender`) (make `Color` 0 0 255 255))))