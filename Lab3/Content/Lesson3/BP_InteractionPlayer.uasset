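; VR player Blueprint for a gaze-aimed shooting game where pressing the Act input scores points.
; Act plays a sound and line-traces from the VR camera, calling InteractMessage on the hit actor to get points.
; Nonzero points update the BP_Scoreboard found at BeginPlay, spawn a BP_ScoreAddition at the hit and play a sound at the board.
; Tick repeats the trace, placing the Reticle at its end point.
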(event `InputAction|InputAction Act`
  (params (Key :type "Key Structure" :default "AnyKey"))
  (bind _scoreboard (`self.Scoreboard`))
  (:`Pressed`
    (bind (_location _forward_vector) (`/Game/LayoutAssets/Utility/LayoutVRUtilityFunctions.Get Player VR Camera Properties`))
    (`GameplayStatics.SpawnSoundAtLocation` "/Game/LayoutAssets/Sounds/SoundWaves/SW_Bongo.SW_Bongo" _location)
    (bind (_outhit _returnvalue) (`KismetSystemLibrary.LineTraceSingle` _location (+ _location (* _forward_vector 10000)) "TraceTypeQuery1"))
    (if _returnvalue
      (bind (_bblockinghit _binitialoverlap _time _location_2 _impactpoint _normal _impactnormal _physmat _hitactor) (`GameplayStatics.BreakHitResult` _outhit))
      (bind _score (message `/Game/Lesson3/BPI_Interaction.Interact` _hitactor))
      ;[1 1 1] Prevent score addition if hitting wall or cover
      (if (not (== _score 0))
        (bind _output_get (set `self.Score` (+ (`self.Score`) _score)))
        (`/Game/Lesson3/BP_Scoreboard.UpdateScore` _scoreboard _output_get)
        (`|SpawnActorFromClass` "/Game/LayoutAssets/Blueprints/BP_ScoreAddition.BP_ScoreAddition_C" (`KismetMathLibrary.MakeTransform` _location_2 (struct) (2.0 2.0 2.0)) "Undefined" "OverrideRootScale" null _score)
        (`GameplayStatics.SpawnSoundAtLocation` "/Game/LayoutAssets/Sounds/SoundWaves/SW_ElectronicSnare.SW_ElectronicSnare" (`self.K2_GetActorLocation` _scoreboard))))))

(event `self.ReceiveBeginPlay`
  (bind _outactors (`GameplayStatics.GetAllActorsOfClass` "/Game/Lesson3/BP_Scoreboard.BP_Scoreboard_C"))
  (set `self.Scoreboard` (`KismetArrayLibrary.Array_Get` _outactors)))

(event `self.ReceiveTick`
  (params (DeltaSeconds :type "Float (single-precision)"))
  (bind (_location _forward_vector) (`/Game/LayoutAssets/Utility/LayoutVRUtilityFunctions.Get Player VR Camera Properties`))
  (bind _outhit (`KismetSystemLibrary.LineTraceSingle` _location (+ _location (* _forward_vector 10000)) "TraceTypeQuery1"))
  (`SceneComponent.K2_SetWorldLocation` (`self.Reticle`) (`.TraceEnd` (`GameplayStatics.BreakHitResult` _outhit)) false false))

(fn `UserConstructionScript`)