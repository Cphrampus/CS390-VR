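; BP_Target_Rotate is a target actor that jitters around its spawn point and respawns elsewhere when hit through Interact.
; After a random startup delay, the Rotate timeline scales a freshly randomized offset each update, moving the actor's location without changing its rotation.
; Interact spawns an explosion, destroys the actor, spawns a replacement at a random position on a fixed-X plane and returns a constant, likely points.
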(event `self.ReceiveBeginPlay`
  (set `self.Origin` (`self.K2_GetActorLocation`))
  (`KismetSystemLibrary.Delay` (`KismetMathLibrary.RandomFloatInRange` 0.0 2.0))
  (bind (_direction _data) (`Timeline|Rotate` :!via `PlayFromStart`)
    (:`Update`
      (`self.K2_SetActorLocation` (+ (`self.Origin`) (* (`KismetMathLibrary.MakeVector` (`KismetMathLibrary.RandomFloatInRange` -10.0 0.0) (`KismetMathLibrary.RandomFloatInRange` -10.0 10.0) (`KismetMathLibrary.RandomFloatInRange` -20.0 20.0)) _data))))))

(event `self.ReceiveActorBeginOverlap`
  (params (OtherActor :type "Actor Object Reference")))

(event `self.ReceiveTick`
  (params (DeltaSeconds :type "Float (single-precision)")))

(fn `Interact`
  (returns (Score :type Integer))
  (`GameplayStatics.SpawnEmitterAtLocation` "/Game/MobileStarterContent/Particles/P_Explosion.P_Explosion" (`self.K2_GetActorLocation`))
  (`self.K2_DestroyActor`)
  (`|SpawnActorFromClass` "BP_Target_Rotate_C" (`KismetMathLibrary.MakeTransform` (`KismetMathLibrary.MakeVector` 1350.0 (`KismetMathLibrary.RandomFloatInRange` -1956.0 -96.0) (`KismetMathLibrary.RandomFloatInRange` 110.0 400.0))) "Undefined" "OverrideRootScale")
  (return 10))

(fn `UserConstructionScript`)