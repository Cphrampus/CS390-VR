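; Shooting-gallery style target actor that randomly switches between blue, gold and red, each worth a different score, with red negative.
; ChangeType sets the material and Value, then re-calls itself after a random delay, starting from BeginPlay.
; Interact plays a random explosion, independent of the current color, destroys the target, spawns a replacement at a random position on a fixed X plane, and returns Value.
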(event `ChangeType`
  (bind _target (`self.Target`))
  (switch `int` (`KismetMathLibrary.RandomIntegerInRange` 0 2)
    (:`0`
      (`PrimitiveComponent.SetMaterial` _target 0 "/Game/Lesson3/Materials/Targets/MI_Targets_Blue.MI_Targets_Blue")
      (set `self.Value` 5))
    (:`1`
      (`PrimitiveComponent.SetMaterial` _target 0 "/Game/Lesson3/Materials/Targets/MI_Targets_Gold.MI_Targets_Gold")
      (set `self.Value` 10))
    (:`2`
      (`PrimitiveComponent.SetMaterial` _target 0 "/Game/Lesson3/Materials/Targets/MI_Targets_Red.MI_Targets_Red")
      (set `self.Value` -5)))
  (`KismetSystemLibrary.Delay` (`KismetMathLibrary.RandomFloatInRange` 2.0 6.0))
  (`self.ChangeType`))

(event `self.ReceiveBeginPlay`
  (`self.ChangeType`))

(event `self.ReceiveActorBeginOverlap`
  (params (OtherActor :type "Actor Object Reference")))

(event `self.ReceiveTick`
  (params (DeltaSeconds :type "Float (single-precision)")))

(fn `Interact`
  (returns (Score :type Integer))
  (bind _returnvalue (`self.K2_GetActorLocation`))
  (switch `int` (`KismetMathLibrary.RandomIntegerInRange` 0 2)
    (:`0`
      (`GameplayStatics.SpawnEmitterAtLocation` "/Game/Lesson3/Effects/P_NeonExplosion_Blue.P_NeonExplosion_Blue" _returnvalue))
    (:`1`
      (`GameplayStatics.SpawnEmitterAtLocation` "/Game/Lesson3/Effects/P_NeonExplosion_Green.P_NeonExplosion_Green" _returnvalue))
    (:`2`
      (`GameplayStatics.SpawnEmitterAtLocation` "/Game/Lesson3/Effects/P_NeonExplosion_Red.P_NeonExplosion_Red" _returnvalue)))
  (`self.K2_DestroyActor`)
  (`|SpawnActorFromClass` "BP_Target_ColorChange_C" (`KismetMathLibrary.MakeTransform` (`KismetMathLibrary.MakeVector` 1350.0 (`KismetMathLibrary.RandomFloatInRange` -1956.0 -96.0) (`KismetMathLibrary.RandomFloatInRange` 110.0 400.0))) "Undefined" "OverrideRootScale")
  (return (`self.Value`)))

(fn `UserConstructionScript`)