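; BP_Target_PopUp is a target actor that pops up after a random delay and explodes when interacted with.
; A timeline started after BeginPlay's delay offsets it vertically from its stored origin.
; Interact plays a randomly colored neon explosion, spawns a replacement at the origin, destroys itself and returns a fixed integer.
; Each replacement restarts the cycle with a new random delay.
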(event `self.ReceiveBeginPlay`
  (set `self.Origin` (`self.K2_GetActorLocation`))
  (`KismetSystemLibrary.Delay` (`KismetMathLibrary.RandomFloatInRange` 2.0 8.0))
  (bind (_direction _data) (`Timeline|UpAndDown` :!via `PlayFromStart`)
    (:`Update`
      (`self.K2_SetActorLocation` (+ (`self.Origin`) (* (0.0 0.0 200.0) _data))))))

(event `self.ReceiveActorBeginOverlap`
  (params (OtherActor :type "Actor Object Reference")))

(event `self.ReceiveTick`
  (params (DeltaSeconds :type "Float (single-precision)")))

(fn `Interact`
  (returns (Score :type Integer))
  (bind _returnvalue (`self.K2_GetActorLocation`))
  (switch `int` (`KismetMathLibrary.RandomIntegerInRange` 0 2)
    (:`0`
      (`GameplayStatics.SpawnEmitterAtLocation` "/Game/Lesson3/Effects/P_NeonExplosion_Green.P_NeonExplosion_Green" _returnvalue))
    (:`1`
      (`GameplayStatics.SpawnEmitterAtLocation` "/Game/Lesson3/Effects/P_NeonExplosion_Blue.P_NeonExplosion_Blue" _returnvalue))
    (:`2`
      (`GameplayStatics.SpawnEmitterAtLocation` "/Game/Lesson3/Effects/P_NeonExplosion_Red.P_NeonExplosion_Red" _returnvalue)))
  (`|SpawnActorFromClass` "BP_Target_PopUp_C" (`KismetMathLibrary.MakeTransform` (`self.Origin`)) "Undefined" "OverrideRootScale")
  (`self.K2_DestroyActor`)
  (return 5))

(fn `UserConstructionScript`)