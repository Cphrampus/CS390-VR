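; BP_VRCamera is a stationary camera actor for VR that can fade the view to and from black.
; Each tick it offsets its stored starting transform by the headset pose, or rotates to face the player pawn when no HMD is enabled.
; Fade events play timelines that drive the Opacity of a dynamic M_Fade material on its BlindingBox.
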(event `FadeFromBlack`
  ;[1 1 1] Fade from Black
  (bind _returnvalue (`PrimitiveComponent.CreateDynamicMaterialInstance` (`self.BlindingBox`) 0 "/Game/Materials/UI/M_Fade.M_Fade"))
  (set `self.FadeDMI` _returnvalue)
  (bind (_direction _data) (`Timeline|FadeIn` :!via `PlayFromStart`)
    (:`Update`
      (`MaterialInstanceDynamic.SetScalarParameterValue` (`self.FadeDMI`) "Opacity" _data))))

(event `FadeToBlack`
  ;[1 1 1] Fade to Black
  (bind _returnvalue (`PrimitiveComponent.CreateDynamicMaterialInstance` (`self.BlindingBox`) 0 "/Game/Materials/UI/M_Fade.M_Fade"))
  (set `self.FadeDMI` _returnvalue)
  (bind (_direction _data) (`Timeline|FadeOut` :!via `PlayFromStart`)
    (:`Update`
      (`MaterialInstanceDynamic.SetScalarParameterValue` (`self.FadeDMI`) "Opacity" _data))))

(event `self.ReceiveTick`
  (params (DeltaSeconds :type "Float (single-precision)"))
  (if (`HeadMountedDisplayFunctionLibrary.IsHeadMountedDisplayEnabled`)
    (bind _newtransform (`/Game/Blueprints/Utility/LayoutVRUtilityFunctions.TransformWithHMD` (`self.InitialTransform`)))
    (`self.K2_SetActorLocationAndRotation` (.location _newtransform) (.rotation _newtransform))
    (else
      (`self.SetActorRotation` (`KismetMathLibrary.FindLookAtRotation` (`self.K2_GetActorLocation`) (`self.K2_GetActorLocation` (`GameplayStatics.GetPlayerPawn` 0)))))))

(event `self.ReceiveBeginPlay`
  (set `self.InitialTransform` (`self.GetTransform`)))

(fn `UserConstructionScript`
  (bind _returnvalue (`PrimitiveComponent.CreateDynamicMaterialInstance` (`self.BlindingBox`) 0 null))
  (set `self.FadeDMI` _returnvalue))